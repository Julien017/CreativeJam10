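; Cannon actor that players push along a spline, load with projectiles and fire.
; Side overlap counts drive its spline position each tick, paused while loading; other colliders register it on PlayerCharacterBP or toggle tooltips.
; LoadCanon stores the projectile class, StartActivateCanon arms firing and ActivateCanon spawns the projectile.
; Explosive rounds start a timer that, unless cleared by firing, explodes, empties and temporarily disables the cannon.
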(event OnComponentBeginOverlap(LeftMovementCollider)
  (params (OverlappedComponent :type Primitive%20Component%20Object%20Reference) (OtherActor :type Actor%20Object%20Reference) (OtherComp :type Primitive%20Component%20Object%20Reference) (OtherBodyIndex :type Integer) (bFromSweep :type Boolean) (SweepResult :type Hit%20Result%20Structure%20%28by%20ref%29))
  (bind _asplayer_character_bp (Utilities|Casting|CastToPlayerCharacterBP OtherActor))
  (Variables|/Game/Blueprints/Players/PlayerCharacterBP.PlayerCharacterBP_C|SetIsReadyToPush _asplayer_character_bp true)
  (Math|Integer|IncrementInt (Variables|Default|GetLeftSideCollisionNumber)))

(event OnComponentBeginOverlap(RightMovementCollider)
  (params (OverlappedComponent :type Primitive%20Component%20Object%20Reference) (OtherActor :type Actor%20Object%20Reference) (OtherComp :type Primitive%20Component%20Object%20Reference) (OtherBodyIndex :type Integer) (bFromSweep :type Boolean) (SweepResult :type Hit%20Result%20Structure%20%28by%20ref%29))
  (bind _asplayer_character_bp (Utilities|Casting|CastToPlayerCharacterBP OtherActor))
  (Variables|/Game/Blueprints/Players/PlayerCharacterBP.PlayerCharacterBP_C|SetIsReadyToPush _asplayer_character_bp true)
  (Math|Integer|IncrementInt (Variables|Default|GetRightSideCollisionNumber)))

(event OnComponentEndOverlap(LeftMovementCollider)
  (params (OverlappedComponent :type Primitive%20Component%20Object%20Reference) (OtherActor :type Actor%20Object%20Reference) (OtherComp :type Primitive%20Component%20Object%20Reference) (OtherBodyIndex :type Integer))
  (bind _asplayer_character_bp (Utilities|Casting|CastToPlayerCharacterBP OtherActor))
  (Variables|/Game/Blueprints/Players/PlayerCharacterBP.PlayerCharacterBP_C|SetIsReadyToPush _asplayer_character_bp false)
  (Math|Integer|DecrementInt (Variables|Default|GetLeftSideCollisionNumber)))

(event OnComponentBeginOverlap(TooltipLoadCollision)
  (params (OverlappedComponent :type Primitive%20Component%20Object%20Reference) (OtherActor :type Actor%20Object%20Reference) (OtherComp :type Primitive%20Component%20Object%20Reference) (OtherBodyIndex :type Integer) (bFromSweep :type Boolean) (SweepResult :type Hit%20Result%20Structure%20%28by%20ref%29))
  (Utilities|Casting|CastToPlayerCharacterBP OtherActor)
  (Math|Integer|IncrementInt (Variables|Default|GetTooltipLoadCollisionCount)
    (:%20%20
      (CallFunction|UpdateTooltipLoad))))

(event OnComponentEndOverlap(TooltipLoadCollision)
  (params (OverlappedComponent :type Primitive%20Component%20Object%20Reference) (OtherActor :type Actor%20Object%20Reference) (OtherComp :type Primitive%20Component%20Object%20Reference) (OtherBodyIndex :type Integer))
  (Utilities|Casting|CastToPlayerCharacterBP OtherActor)
  (Math|Integer|DecrementInt (Variables|Default|GetTooltipLoadCollisionCount)
    (:%20%20
      (CallFunction|UpdateTooltipLoad))))

(event OnComponentEndOverlap(ActivationCollider)
  (params (OverlappedComponent :type Primitive%20Component%20Object%20Reference) (OtherActor :type Actor%20Object%20Reference) (OtherComp :type Primitive%20Component%20Object%20Reference) (OtherBodyIndex :type Integer))
  (bind _asplayer_character_bp (Utilities|Casting|CastToPlayerCharacterBP OtherActor))
  (Variables|/Game/Blueprints/Players/PlayerCharacterBP.PlayerCharacterBP_C|SetCurrentCanonToActivate _asplayer_character_bp 0))

(event OnComponentEndOverlap(RightMovementCollider)
  (params (OverlappedComponent :type Primitive%20Component%20Object%20Reference) (OtherActor :type Actor%20Object%20Reference) (OtherComp :type Primitive%20Component%20Object%20Reference) (OtherBodyIndex :type Integer))
  (bind _asplayer_character_bp (Utilities|Casting|CastToPlayerCharacterBP OtherActor))
  (Variables|/Game/Blueprints/Players/PlayerCharacterBP.PlayerCharacterBP_C|SetIsReadyToPush _asplayer_character_bp false)
  (Math|Integer|DecrementInt (Variables|Default|GetRightSideCollisionNumber)))

(event OnComponentBeginOverlap(ActivationCollider)
  (params (OverlappedComponent :type Primitive%20Component%20Object%20Reference) (OtherActor :type Actor%20Object%20Reference) (OtherComp :type Primitive%20Component%20Object%20Reference) (OtherBodyIndex :type Integer) (bFromSweep :type Boolean) (SweepResult :type Hit%20Result%20Structure%20%28by%20ref%29))
  (bind _asplayer_character_bp (Utilities|Casting|CastToPlayerCharacterBP OtherActor))
  (Variables|/Game/Blueprints/Players/PlayerCharacterBP.PlayerCharacterBP_C|SetCurrentCanonToActivate _asplayer_character_bp self))

(event OnComponentBeginOverlap(TooltipFireCollision)
  (params (OverlappedComponent :type Primitive%20Component%20Object%20Reference) (OtherActor :type Actor%20Object%20Reference) (OtherComp :type Primitive%20Component%20Object%20Reference) (OtherBodyIndex :type Integer) (bFromSweep :type Boolean) (SweepResult :type Hit%20Result%20Structure%20%28by%20ref%29))
  (Utilities|Casting|CastToPlayerCharacterBP OtherActor)
  (Math|Integer|IncrementInt (Variables|Default|GetTooltipFireCollisionCount)
    (:%20%20
      (CallFunction|UpdateTooltipFire))))

(event OnComponentEndOverlap(TooltipFireCollision)
  (params (OverlappedComponent :type Primitive%20Component%20Object%20Reference) (OtherActor :type Actor%20Object%20Reference) (OtherComp :type Primitive%20Component%20Object%20Reference) (OtherBodyIndex :type Integer))
  (Utilities|Casting|CastToPlayerCharacterBP OtherActor)
  (Math|Integer|DecrementInt (Variables|Default|GetTooltipFireCollisionCount)
    (:%20%20
      (CallFunction|UpdateTooltipFire))))

(event OnComponentBeginOverlap(LoadCanonCollider)
  (params (OverlappedComponent :type Primitive%20Component%20Object%20Reference) (OtherActor :type Actor%20Object%20Reference) (OtherComp :type Primitive%20Component%20Object%20Reference) (OtherBodyIndex :type Integer) (bFromSweep :type Boolean) (SweepResult :type Hit%20Result%20Structure%20%28by%20ref%29))
  (bind _asplayer_character_bp (Utilities|Casting|CastToPlayerCharacterBP OtherActor))
  (Variables|/Game/Blueprints/Players/PlayerCharacterBP.PlayerCharacterBP_C|SetCurrentCanonToLoad _asplayer_character_bp self))

(event OnComponentEndOverlap(LoadCanonCollider)
  (params (OverlappedComponent :type Primitive%20Component%20Object%20Reference) (OtherActor :type Actor%20Object%20Reference) (OtherComp :type Primitive%20Component%20Object%20Reference) (OtherBodyIndex :type Integer))
  (bind _asplayer_character_bp (Utilities|Casting|CastToPlayerCharacterBP OtherActor))
  (Variables|/Game/Blueprints/Players/PlayerCharacterBP.PlayerCharacterBP_C|SetCurrentCanonToLoad _asplayer_character_bp 0))

(event Custom|UpdateTooltipFire
  (Rendering|SetVisibility (Variables|Default|GetTooltipFire) (>= (Variables|Default|GetTooltipFireCollisionCount) 1) false))

(event Custom|UpdateTooltipLoad
  (Rendering|SetVisibility (Variables|Default|GetTooltipLoad) (>= (Variables|Default|GetTooltipLoadCollisionCount) 1) false))

(event EventBeginPlay
  (CallFunction|UpdateCanonPosition)
  (Widget|Transform|SetRenderScale (UserInterface|GetUserWidgetObject (Variables|Default|GetTooltipLoad)) "(X=0.200000,Y=0.200000)")
  (CallFunction|UpdateTooltipLoad)
  (Widget|Transform|SetRenderScale (UserInterface|GetUserWidgetObject (Variables|Default|GetTooltipFire)) "(X=0.200000,Y=0.200000)")
  (CallFunction|UpdateTooltipFire))

(event Collision|EventActorBeginOverlap
  (params (OtherActor :type Actor%20Object%20Reference)))

(event EventTick
  (params (DeltaSeconds :type Float%20%28single-precision%29))
  (CallFunction|UpdateCanonTimeonSpline DeltaSeconds)
  (CallFunction|UpdateCanonPosition))

(fn ConstructionScript)

(fn UpdateCanonPosition
  (Transformation|SetWorldLocation (Variables|Default|GetCanonRoot) (Spline|GetLocationatTime (Variables|Default|GetCanonTrail) (Variables|Default|GetTimeOnSpline) "World" false) false false))

(fn UpdateCanonTimeonSpline
  (params (DeltaTime :type Float%20%28single-precision%29))
  (if (not (Variables|Default|GetIsLoading))
    (if (or (Variables|Default|GetIsLoaded) (not (Variables|Default|GetIsEnabled)))
      (LocalVariables|SetCurrentSpeedMultiplier (Variables|Default|GetLoadedCanonSpeedMultiplier)))
    (Variables|Default|SetTimeOnSpline (Math|Float|Clamp(Float) (+ (* (+ (* (Variables|Default|GetRightSideCollisionNumber) -1.0) (Math|Conversions|ToFloat(Integer) (Variables|Default|GetLeftSideCollisionNumber))) (Variables|Default|GetMovingSpeed) DeltaTime (LocalVariables|GetCurrentSpeedMultiplier)) (Variables|Default|GetTimeOnSpline))))))

(fn ActivateCanon
  (CallFunction|SpawnProjectile)
  (Utilities|Time|ClearandInvalidateTimerbyHandle (Variables|Default|GetCanonExplosionTimer))
  (Variables|Default|SetShouldFire false))

(fn SpawnProjectile
  (Game|SpawnActorfromClass (Variables|Default|GetProjectileClass) (Transformation|GetWorldTransform (Variables|Default|GetProjectileSpawnArrow)) "AdjustIfPossibleButAlwaysSpawn" 0 1.5e+03 0))

(fn LoadCanon
  (params (ProjectileType :type Base%20Projectile%20BP%20Class%20Reference) (TimeBeforeExplosion :type Float%20%28single-precision%29))
  (bind _output_get (Variables|Default|SetProjectileClass ProjectileType))
  (if (Utilities|ClassIsChildOf _output_get "/Game/Blueprints/Projectiles/ExplosiveProjectileBP.ExplosiveProjectileBP_C")
    (bind _returnvalue (Utilities|Time|SetTimerbyFunctionName 0 "Explode" (+ TimeBeforeExplosion (Variables|Default|GetBombExtraTimeBeforeExplosion))))
    (Variables|Default|SetCanonExplosionTimer _returnvalue))
  (if (Variables|Default|GetIsLoaded)
    (return false)
    (else
      (bind _output_get_2 (Variables|Default|SetIsLoaded true))
      (Variables|Default|SetIsLoading false)
      (return _output_get_2))))

(fn Explode
  (Effects|SpawnEmitteratLocation "/Game/StarterContent/Particles/P_BiggerExplosion.P_BiggerExplosion" (Transformation|GetWorldLocation (Variables|Default|GetCanonRoot)))
  (CallFunction|DisableCanon))

(fn DisableCanon
  (Variables|Default|SetIsEnabled false)
  (Utilities|Time|SetTimerbyFunctionName self "EnableCanon" (Variables|Default|GetExplosionStuntDuration))
  (Variables|Default|SetProjectileClass 0)
  (Variables|Default|SetIsLoaded false))

(fn EnableCanon
  (Variables|Default|SetIsEnabled true))

(fn StartActivateCanon
  (if (Variables|Default|GetIsLoaded)
    (Variables|Default|SetIsLoaded false)
    (Variables|Default|SetShouldFire true)
    (return true)
    (else
      (return false))))

(fn InitiateLoading
  (Variables|Default|SetIsLoading true))