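; PlayerZoneFront is a zone actor with an Area box that positions explosive ammo spawns relative to destroyed projectiles.
; SpawnBomb keeps the destroyed projectile's X and takes random Y and Z from within the box.
; It adds the DistanceFromPlayerZoneToSpawnBomb offset and spawns ExplosiveAmmo there, ignoring collisions.
; The event graph and construction script are empty, so SpawnBomb relies on external callers.
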(event OnComponentBeginOverlap(Area)
  (params (OverlappedComponent :type Primitive%20Component%20Object%20Reference) (OtherActor :type Actor%20Object%20Reference) (OtherComp :type Primitive%20Component%20Object%20Reference) (OtherBodyIndex :type Integer) (bFromSweep :type Boolean) (SweepResult :type Hit%20Result%20Structure%20%28by%20ref%29)))

(event EventBeginPlay)

(event Collision|EventActorBeginOverlap
  (params (OtherActor :type Actor%20Object%20Reference)))

(event EventTick
  (params (DeltaSeconds :type Float%20%28single-precision%29)))

(fn ConstructionScript)

(fn SpawnBomb
  (params (DestroyedProjectilePos :type Vector))
  (bind _area (Variables|Default|GetArea))
  (bind _returnvalue (Transformation|GetWorldLocation _area))
  (bind _boxextent (Variables|/Script/Engine.BoxComponent|GetBoxExtent _area))
  (bind _returnvalue_2 (Math|Random|RandomPointinBoundingBox _returnvalue _boxextent))
  (bind (_x _y _z) (Math|Vector|BreakVector _returnvalue_2))
  (bind _output_get (LocalVariables|SetTargetLocation (Math|Vector|MakeVector (.X (Math|Vector|BreakVector DestroyedProjectilePos)) _y _z)))
  (Game|SpawnActorfromClass "/Game/Blueprints/Projectiles/ExplosiveAmmo.ExplosiveAmmo_C" (Math|Transform|MakeTransform (+ _output_get (Variables|Default|GetDistanceFromPlayerZoneToSpawnBomb)) "0, 0, 0" "1,1,1") "AlwaysSpawn" 0 0))