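; An actor that carries a widget tooltip and keeps it at an offset from a target actor.
; A looping timer started on BeginPlay teleports it to the target's location plus the offset at a configurable interval, instead of using Tick.
; It destroys itself if the target becomes invalid after having been valid, so it tolerates a target assigned late.
; UpdateTooltip toggles the widget's visibility.
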(event Custom|Follow
  (Utilities|IsValid (Variables|Default|GetTarget)
    (:Is%20Valid
      (Variables|Default|SetHasBeenValid true)
      (Transformation|SetActorLocation (+ (Transformation|GetActorLocation (Variables|Default|GetTarget)) (Variables|Default|GetDeltaPosition)) false true))
    (:Is%20Not%20Valid
      (if (Variables|Default|GetHasBeenValid)
        (Actor|DestroyActor)))))

(event Custom|UpdateTooltip
  (params (Visibility :type Boolean))
  (Rendering|SetVisibility (Variables|Default|GetWidget) Visibility false))

(event EventBeginPlay
  (Utilities|Time|SetTimerbyEvent (delegate Custom|Follow) (Variables|Default|GetFollowUpdateFrequency) true))

(event Collision|EventActorBeginOverlap
  (params (OtherActor :type Actor%20Object%20Reference)))

(event EventTick
  (params (DeltaSeconds :type Float%20%28single-precision%29)))

(fn ConstructionScript)