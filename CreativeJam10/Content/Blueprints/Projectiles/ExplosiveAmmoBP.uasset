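; ExplosiveAmmoBP is a timed explosive projectile that loses speed when it hits something.
; On BeginPlay it starts a timer that calls DestroyProjectile, which is not defined in this graph, after TimeBeforeExplosion.
; Each collision hit divides the physics linear velocity by GroundVelocityDivider, damping its motion until the timer fires.
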(event OnComponentHit(Collision)
  (params (HitComponent :type Primitive%20Component%20Object%20Reference) (OtherActor :type Actor%20Object%20Reference) (OtherComp :type Primitive%20Component%20Object%20Reference) (NormalImpulse :type Vector :default "0, 0, 0") (Hit :type Hit%20Result%20Structure%20%28by%20ref%29))
  (bind _collision (Variables|Default|GetCollision))
  (bind _returnvalue (Physics|GetPhysicsLinearVelocity _collision "None"))
  (Physics|SetPhysicsLinearVelocity _collision (/ _returnvalue (Variables|Default|GetGroundVelocityDivider)) false "None"))

(event EventBeginPlay
  (Utilities|Time|SetTimerbyFunctionName self "DestroyProjectile" (Variables|Default|GetTimeBeforeExplosion)))

(event Collision|EventActorBeginOverlap
  (params (OtherActor :type Actor%20Object%20Reference)))

(event EventTick
  (params (DeltaSeconds :type Float%20%28single-precision%29)))

(fn ConstructionScript
  (|CallParentFunction))