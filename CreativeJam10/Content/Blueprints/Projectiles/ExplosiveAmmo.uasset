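; ExplosiveAmmo is a bomb projectile that blinks after a delay, then explodes with full radial damage, particles and sound.
; A fast looping timer exponentially raises the blink and emissive parameters on a dynamic material until a threshold triggers DestroyProjectile.
; Collision hits damp physics velocity, with landing and rope-crackle sounds on first impact.
; Attaching to a hand stops projectile movement, and the construction script sizes a dummy sphere to the damage radius.
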(event OnComponentHit(Collision)
  (params (HitComponent :type Primitive%20Component%20Object%20Reference) (OtherActor :type Actor%20Object%20Reference) (OtherComp :type Primitive%20Component%20Object%20Reference) (NormalImpulse :type Vector :default "0, 0, 0") (Hit :type Hit%20Result%20Structure%20%28by%20ref%29))
  (bind _collision (Variables|Default|GetCollision))
  (bind _returnvalue (Physics|GetPhysicsLinearVelocity _collision "None"))
  (Physics|SetPhysicsLinearVelocity _collision (/ _returnvalue (Variables|Default|GetGroundVelocityDivider)) false "None")
  (if (not (Variables|Default|GetIsOnGround))
    (Variables|Default|SetIsOnGround true)
    (Audio|Components|Audio|Play (Variables|Default|GetBombHitGroundSound) 0.0)
    (Audio|Components|Audio|Play (Variables|Default|GetRope_CracklingCue) 0.0)))

(event Custom|StartBlink
  (bind _returnvalue (Utilities|Time|SetTimerbyEvent (delegate Custom|ChangeBlinkValue) 0.002 true))
  (Variables|Default|SetBlinkTimer _returnvalue))

(event Custom|ChangeBlinkValue
  (bind _dynamicmat (Variables|Default|GetDynamicMat))
  (Rendering|Material|SetScalarParameterValue _dynamicmat "BlinkFactor" (Variables|Default|GetBlinkSpeedMultiplier) :!class /Script/Engine.MaterialInstanceDynamic)
  (Rendering|Material|SetScalarParameterValue _dynamicmat "EmissiveValue" (* (Variables|Default|GetBlinkSpeedMultiplier) 1.05) :!class /Script/Engine.MaterialInstanceDynamic)
  (Variables|Default|SetBlinkSpeedMultiplier (* (Variables|Default|GetBlinkSpeedMultiplier) 1.0002))
  (if (< (Variables|Default|GetMaxBlinkMultiplier) (Variables|Default|GetBlinkSpeedMultiplier))
    (Utilities|Time|InvalidateTimerHandle (Variables|Default|GetBlinkTimer))
    (CallFunction|DestroyProjectile)))

(event EventBeginPlay
  (Utilities|Time|SetTimerbyEvent (delegate Custom|StartBlink) (Variables|Default|GetTimeBeforeBlink))
  (|CallParentFunction))

(event Collision|EventActorBeginOverlap
  (params (OtherActor :type Actor%20Object%20Reference)))

(event EventAttachtoHand
  (params (SkeletalMeshComponent :type Skeletal%20Mesh%20Component%20Object%20Reference))
  (Game|Components|ProjectileMovement|StopSimulating (Variables|Default|GetProjectileMovement) (Collision|MakeHitResult false false 0.0 "0, 0, 0" "0, 0, 0" "0,0,1" "0,0,1" 0 0 0 "None" 0 0 "0, 0, 0" "0, 0, 0"))
  (|CallParentFunction SkeletalMeshComponent))

(event EventTick
  (params (DeltaSeconds :type Float%20%28single-precision%29)))

(fn ConstructionScript
  (Components|Sphere|SetSphereRadius (Variables|Default|GetCollisionSphereDummy) (Variables|Default|GetDamageRadius) true)
  (bind _returnvalue (Rendering|Material|CreateDynamicMaterialInstance (Variables|Default|GetSphere) 0 "/Game/Assets/Bombe/M_BlinkingBomb.M_BlinkingBomb" :!class /Script/Engine.PrimitiveComponent))
  (Variables|Default|SetDynamicMat _returnvalue)
  (|CallParentFunction))

(fn DestroyProjectile
  (bind _returnvalue (Transformation|GetActorLocation))
  (Effects|SpawnEmitteratLocation "/Game/StarterContent/Particles/P_BiggerExplosion.P_BiggerExplosion" _returnvalue)
  (Game|Damage|ApplyRadialDamage 1.0 _returnvalue (Variables|Default|GetDamageRadius) 0 0 self 0 true "ECC_WorldStatic")
  (Audio|PlaySound2D "/Game/Audio/Cue/ExplosionCue.ExplosionCue")
  (Actor|DestroyActor))