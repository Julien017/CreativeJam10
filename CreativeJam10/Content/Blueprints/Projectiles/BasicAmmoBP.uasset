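; BasicAmmoBP is an ammo actor that can ride a dispenser spline or be attached to a hand.
; BeginPlay turns off physics simulation on its collision before running the parent logic.
; While in the dispenser, Tick advances a clamped progress value, moves the actor along the spline and destroys it at the end.
; Attaching to a hand clears the dispenser state, stopping that movement, and defers to the parent.
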(event EventBeginPlay
  (Physics|SetSimulatePhysics (Variables|Default|GetCollision) false)
  (|CallParentFunction))

(event Collision|EventActorBeginOverlap
  (params (OtherActor :type Actor%20Object%20Reference)))

(event EventAttachtoHand
  (params (SkeletalMeshComponent :type Skeletal%20Mesh%20Component%20Object%20Reference))
  (Variables|Default|SetInDispenser false)
  (|CallParentFunction SkeletalMeshComponent))

(event EventTick
  (params (DeltaSeconds :type Float%20%28single-precision%29))
  (if (Variables|Default|GetInDispenser)
    (bind _output_get (Variables|Default|SetDispenserProgress (Math|Float|Min(Float) (+ (Variables|Default|GetDispenserProgress) (* (Variables|Default|GetDispenserBallSpeed) DeltaSeconds)) 1.0)))
    (Transformation|SetActorLocation (Spline|GetLocationatTime (Variables|Default|GetSplineComponent) _output_get "World" false) false false)
    (if (== (Variables|Default|GetDispenserProgress) 1.0)
      (Actor|DestroyActor))))

(fn ConstructionScript
  (|CallParentFunction))