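; Enemy wave manager that runs a sequence of phases from BeginPlay and prints a win once all are cleared.
; The construction script divides the Area box into evenly spaced straight spline lanes.
; Each phase spawns classic or trebuchet enemies on a looping timer at random lanes, trebuchets midway between two neighbours, and advances when its kill count runs out.
; Helper functions convert progress along a lane into world positions.
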(event Custom|StartNewPhase
  (bind _phasedata (CallFunction|GetCurrentPhase))
  (Development|PrintString "Starting New Phase")
  (bind _result (Math|Integer|IncrementInt (Variables|Phase|GetPhaseIndex))
    (:%20%20
      (if (>= _result (Utilities|Array|Length (Variables|Phase|GetPhases)))
        (Development|PrintString "Win")
        (else
          (bind _output_get (Variables|Default|SetEnemiesLeftToKill (.enemiescount _phasedata)))
          (Variables|Default|SetEnemiesLeftToSpawn _output_get)
          (bind _returnvalue (Utilities|Time|SetTimerbyEvent (delegate Custom|SpawnEnemy) (.delaybetweenspawns _phasedata) true))
          (Variables|Default|SetSpawnTimerHandle _returnvalue))))))

(event Custom|EnemyKilled
  (bind _result (Math|Integer|DecrementInt (Variables|Default|GetEnemiesLeftToKill))
    (:%20%20
      (if (== _result 0)
        (CallFunction|StartNewPhase)))))

(event Custom|SpawnEnemy
  (bind _enemytype (CallFunction|GetRandomEnemyType))
  (switch int _enemytype
    (:0
      (bind (_worldtransform _laneindex) (CallFunction|GetClassicEnemySpawningLane))
      (bind _returnvalue (Game|SpawnActorfromClass "/Game/Blueprints/Enemies/EnemyClassicBP.EnemyClassicBP_C" _worldtransform "AlwaysSpawn" 0 0))
      (Variables|/Game/Blueprints/Enemies/EnemyBP.EnemyBP_C|SetLaneIndex _returnvalue _laneindex)
      (Variables|/Game/Blueprints/Enemies/EnemyBP.EnemyBP_C|SetWarzone _returnvalue self)
      (Variables|/Game/Blueprints/Enemies/EnemyBP.EnemyBP_C|SetTimeToEndFactor _returnvalue (.timetoreachendfactor (CallFunction|GetCurrentPhase))))
    (:1
      (bind (_worldtransform_2 _laneindex_2) (CallFunction|GetTrebuchetEnemySpawningLane))
      (bind _returnvalue_2 (Game|SpawnActorfromClass "/Game/Blueprints/Enemies/EnemyTrebuchetBP.EnemyTrebuchetBP_C" _worldtransform_2 "AlwaysSpawn" 0 0))
      (Variables|/Game/Blueprints/Enemies/EnemyBP.EnemyBP_C|SetLaneIndex _returnvalue_2 _laneindex_2)
      (Variables|/Game/Blueprints/Enemies/EnemyBP.EnemyBP_C|SetWarzone _returnvalue_2 self)
      (Variables|/Game/Blueprints/Enemies/EnemyBP.EnemyBP_C|SetTimeToEndFactor _returnvalue_2 (.timetoreachendfactor (CallFunction|GetCurrentPhase)))))
  (bind _result (Math|Integer|DecrementInt (Variables|Default|GetEnemiesLeftToSpawn))
    (:%20%20
      (if (== _result 0)
        (Utilities|Time|ClearandInvalidateTimerbyHandle (Variables|Default|GetSpawnTimerHandle))))))

(event Custom|StartSpawning
  (CallFunction|StartNewPhase))

(event EventBeginPlay
  (CallFunction|StartSpawning))

(event Collision|EventActorBeginOverlap
  (params (OtherActor :type Actor%20Object%20Reference)))

(event EventTick
  (params (DeltaSeconds :type Float%20%28single-precision%29)))

(fn ConstructionScript
  (bind _area (Variables|Default|GetArea))
  (bind _area_2 (Variables|Default|GetArea))
  (bind _area_3 (Variables|Default|GetArea))
  (bind _lanescount (Variables|Lanes|GetLanesCount))
  (bind _area_4 (Variables|Default|GetArea))
  (bind _returnvalue (Transformation|GetRelativeTransform _area_3))
  (bind _returnvalue_2 (Math|Conversions|ToFloat(Integer) _lanescount))
  (bind _returnvalue_3 (Transformation|GetRelativeTransform _area_4))
  (bind _boxextent (Variables|/Script/Engine.BoxComponent|GetBoxExtent _area))
  (bind _boxextent_2 (Variables|/Script/Engine.BoxComponent|GetBoxExtent _area_2))
  (bind _returnvalue_4 (* (.x _boxextent) 2.0))
  (bind _returnvalue_5 (/ _returnvalue_4 _returnvalue_2))
  (Utilities|Array|Clear (Variables|Lanes|GetSplines))
  (LocalVariables|SetMinX (- (.x (.location _returnvalue_3)) (.x _boxextent)))
  (LocalVariables|SetMinY (- (.y (.location _returnvalue_3)) (.y _boxextent)))
  (LocalVariables|SetMaxY (+ (.y (.location _returnvalue_3)) (.y _boxextent)))
  (for _index (range 1 (Variables|Lanes|GetLanesCount))
    (bind _returnvalue_6 (AddComponent|AddSplineComponent false (Math|Transform|MakeTransform (Math|Vector|MakeVector (+ (- (* _returnvalue_5 (Math|Conversions|ToFloat(Integer) _index)) (/ _returnvalue_5 2.0)) (LocalVariables|GetMinX)) (.y (.location _returnvalue)) (.z (.location _returnvalue))) (.rotation _returnvalue) (.scale _returnvalue))))
    (Spline|SetLocationatSplinePoint _returnvalue_6 0 (Math|Vector|MakeVector 0.0 (* (.y _boxextent_2) -1.0) 0.0) "Local" true)
    (Spline|SetLocationatSplinePoint _returnvalue_6 1 (Math|Vector|MakeVector 0.0 (.y _boxextent_2) 0.0) "Local" true)
    (Utilities|Array|Add (Variables|Lanes|GetSplines) _returnvalue_6))
  (Development|PrintString "Completed"))

(fn GetRandomEnemyType
  (if (< (Math|Random|RandomFloat) (.trebuchetchance (Utilities|Array|Get(acopy) (Variables|Phase|GetPhases) (Variables|Phase|GetPhaseIndex))))
    ;[1 1 1] SpawnCatapult
    (return 1)
    (else
      ;[1 1 1] Spawn Classic
      (return 0))))

(fn GetClassicEnemySpawningLane
  (bind _lanescount (Variables|Lanes|GetLanesCount))
  (bind _splines (Variables|Lanes|GetSplines))
  (bind _returnvalue (- _lanescount 1))
  (bind _returnvalue_2 (Math|Random|RandomIntegerinRange 0 _returnvalue))
  (bind _output (Utilities|Array|Get(acopy) _splines _returnvalue_2))
  (bind _returnvalue_3 (Transformation|GetWorldTransform _output))
  (return (Math|Transform|MakeTransform (Spline|GetLocationatSplinePoint _output 0 "World") (.rotation _returnvalue_3) (.scale _returnvalue_3)) _returnvalue_2))

(fn GetPositionfromProgression
  (params (Progress :type Float%20%28single-precision%29) (LaneIndex :type Integer))
  (return (Spline|GetLocationatTime (Utilities|Array|Get(acopy) (Variables|Lanes|GetSplines) LaneIndex) Progress "World" false)))

(fn GetCurrentPhase
  (return (Utilities|Array|Get(acopy) (Variables|Phase|GetPhases) (Variables|Phase|GetPhaseIndex))))

(fn GetTrebuchetEnemySpawningLane
  (bind _splines (Variables|Lanes|GetSplines))
  (bind _lanescount (Variables|Lanes|GetLanesCount))
  (bind _returnvalue (- _lanescount 1))
  (bind _returnvalue_2 (Math|Random|RandomIntegerinRange 1 _returnvalue))
  (bind _output (Utilities|Array|Get(acopy) _splines _returnvalue_2))
  (bind _returnvalue_3 (Transformation|GetWorldTransform _output))
  (return (Math|Transform|MakeTransform (Math|Vector|Lerp(Vector) (Spline|GetLocationatSplinePoint _output 0 "World") (Spline|GetLocationatSplinePoint (Utilities|Array|Get(acopy) (Variables|Lanes|GetSplines) (- _returnvalue_2 1)) 0 "World") 0.5) (.rotation _returnvalue_3) (.scale _returnvalue_3)) _returnvalue_2))

(fn GetPositionfromProgressionTrebuchet
  (params (Progress :type Float%20%28single-precision%29) (LaneIndex :type Integer))
  (bind _splines (Variables|Lanes|GetSplines))
  (return (Math|Vector|Lerp(Vector) (Spline|GetLocationatTime (Utilities|Array|Get(acopy) _splines LaneIndex) Progress "World" false) (Spline|GetLocationatTime (Utilities|Array|Get(acopy) _splines (- LaneIndex 1)) Progress "World" false) 0.5)))