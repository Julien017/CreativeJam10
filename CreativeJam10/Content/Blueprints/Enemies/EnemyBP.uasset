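; EnemyBP is an enemy that advances along a Warzone lane toward the gate.
; Tick accumulates time and sets its world location from a clamped time-based progress, which the Warzone converts to a position on its lane index.
; When its capsule overlaps an EndZone, it notifies GameModeBP that an enemy reached the gate, reports itself killed to the Warzone, spawns an explosion and destroys itself.
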(event OnComponentBeginOverlap(Capsule)
  (params (OverlappedComponent :type Primitive%20Component%20Object%20Reference) (OtherActor :type Actor%20Object%20Reference) (OtherComp :type Primitive%20Component%20Object%20Reference) (OtherBodyIndex :type Integer) (bFromSweep :type Boolean) (SweepResult :type Hit%20Result%20Structure%20%28by%20ref%29))
  (Utilities|Casting|CastToEndZone OtherActor)
  (Utilities|FlowControl|Sequence
    (:then_0
      (bind _asgame_mode_bp (Utilities|Casting|CastToGameModeBP (Game|GetGameMode)))
      (Default|EnemyReachedGate _asgame_mode_bp))
    (:then_1
      (Default|EnemyKilled (Variables|Path|GetWarzone)))
    (:then_2
      (Effects|SpawnEmitteratLocation "/Game/StarterContent/Particles/P_Explosion.P_Explosion" (Transformation|GetWorldLocation (Variables|Default|GetDefaultSceneRoot))))
    (:then_3
      (Actor|DestroyActor))))

(event EventBeginPlay)

(event Collision|EventActorBeginOverlap
  (params (OtherActor :type Actor%20Object%20Reference)))

(event EventTick
  (params (DeltaSeconds :type Float%20%28single-precision%29))
  (bind _output_get (Variables|Progress|SetTimeAcc (+ (Variables|Progress|GetTimeAcc) DeltaSeconds)))
  (bind _position (CallFunction|GetPositionfromProgress (Math|Float|Min(Float) (/ _output_get (* (Variables|Progress|GetTimeToEnd) (Variables|Progress|GetTimeToEndFactor))) 1.0)))
  (Transformation|SetWorldLocation (Variables|Default|GetDefaultSceneRoot) _position false false))

(fn ConstructionScript)

(fn GetPositionfromProgress
  (params (Progress :type Float%20%28single-precision%29))
  (bind _position (Default|GetPositionfromProgression (Variables|Path|GetWarzone) Progress (Variables|Path|GetLaneIndex)))
  (return _position))