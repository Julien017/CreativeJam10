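; Game mode Blueprint that tracks health for a gate the player defends against enemies.
; EnemyReachedGate subtracts one Health per call and prints either a warning or, when Health equals exactly zero, a red failure message, with no further game-over logic.
; FixCamera switches the first player controller's view to the CameraActor variable.
; Neither event is called within this graph, and BeginPlay and Tick are unused.
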(event Custom|EnemyReachedGate
  (bind _output_get (Variables|Default|SetHealth (- (Variables|Default|GetHealth) 1.0)))
  (if (== _output_get 0.0)
    (Development|PrintString "YOU FAILED" true true "(R=0.575000,G=0.000000,B=0.010043,A=1.000000)" 1e+01)
    (else
      (Development|PrintString "Enemy reached gate"))))

(event Custom|FixCamera
  (Game|Player|SetViewTargetwithBlend (Game|GetPlayerController 0) (Variables|Default|GetCameraActor) 0.0 "VTBlend_Linear" 0.0 false))

(event EventBeginPlay)

(event EventTick
  (params (DeltaSeconds :type Float%20%28single-precision%29)))

(fn ConstructionScript)